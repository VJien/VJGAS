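; BP_Hero is a hero Blueprint that triggers Gameplay Ability System skills from debug-style key presses.
; Q and Tab send gameplay events to itself tagged Skill4 and Skill3, targeting the first BP_Enemy found in the level, with Q also passing a magnitude.
; Direct ability activation by tag or class and an attribute printout remain as disconnected test nodes, and BeginPlay, Tick and the construction script are empty.
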(event `self.ReceiveTick`
  (params (DeltaSeconds :type "Float (single-precision)")))

(event `Key|Q`
  (params (Key :type "Key Structure"))
  (:`Pressed`
    (bind _outactors (`GameplayStatics.GetAllActorsOfClass` "/Game/VGAS/BP_Enemy.BP_Enemy_C"))
    (`AbilitySystemBlueprintLibrary.SendGameplayEventToActor` self (struct :`TagName` "VG.Skill.Skill4") (make `GameplayEventData` (struct :`TagName` "VG.Skill.Skill4") self (`|GetArrayItem` _outactors) null null (struct) (struct :`GameplayTags` (struct :`(TagName` "VG.Skill.Skill4"))) (struct :`GameplayTags` (struct :`(TagName` "VG.Skill.Skill4"))) 10.0))))

(event `Key|Tab`
  (params (Key :type "Key Structure"))
  (:`Pressed`
    (bind _outactors (`GameplayStatics.GetAllActorsOfClass` "/Game/VGAS/BP_Enemy.BP_Enemy_C"))
    (`AbilitySystemBlueprintLibrary.SendGameplayEventToActor` self (struct :`TagName` "VG.Skill.Skill3") (make `GameplayEventData` (struct :`TagName` "VG.Skill.Skill3") self (`|GetArrayItem` _outactors) null null (struct) (struct :`GameplayTags` (struct :`(TagName` "VG.Skill.Skill3") :`(TagName` "VG.Skill.Skill4"))) (struct :`GameplayTags` (struct :`(TagName` "VG.Skill.Skill3") :`(TagName` "VG.Skill.Skill4")))))))

(fn `UserConstructionScript`)